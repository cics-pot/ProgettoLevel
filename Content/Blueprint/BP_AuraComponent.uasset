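; Unfinished aura Blueprint built around an AuraSphere collision component and a WindEffect Niagara component.
; BeginPlay binds the sphere's end-overlap to an empty handler if the sphere is valid.
; Tick stores WindEffect as NiagaraComp and sets a float camera variable.
; Sphere lookup, begin-overlap binding, Niagara spawning and a zero-force loop over overlapping actors are disconnected, so no aura force is applied.
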(event OnComponentBeginOverlap(AuraSphere)
  (params (OverlappedComponent :type Primitive%20Component%20Object%20Reference) (OtherActor :type Actor%20Object%20Reference) (OtherComp :type Primitive%20Component%20Object%20Reference) (OtherBodyIndex :type Integer) (bFromSweep :type Boolean) (SweepResult :type Hit%20Result%20Structure%20%28by%20ref%29)))

(event OnComponentEndOverlap(AuraSphere)
  (params (OverlappedComponent :type Primitive%20Component%20Object%20Reference) (OtherActor :type Actor%20Object%20Reference) (OtherComp :type Primitive%20Component%20Object%20Reference) (OtherBodyIndex :type Integer)))

(event Custom|CustomEvent_0
  (params (OverlappedComponent :type Primitive%20Component%20Object%20Reference) (OtherActor :type Actor%20Object%20Reference) (OtherComp :type Primitive%20Component%20Object%20Reference) (OtherBodyIndex :type Integer)))

(event Custom|CustomEvent
  (params (OverlappedComponent :type Primitive%20Component%20Object%20Reference) (OtherActor :type Actor%20Object%20Reference) (OtherComp :type Primitive%20Component%20Object%20Reference) (OtherBodyIndex :type Integer) (bFromSweep :type Boolean) (SweepResult :type Hit%20Result%20Structure%20%28by%20ref%29)))

(event EventBeginPlay
  (if (Utilities|IsValid (Variables|Components|GetAura%20Sphere))
    (Collision|BindEventtoOnComponentEndOverlap (Variables|Components|GetAura%20Sphere) (delegate Custom|CustomEvent_0))
    (else
      (bind _output_get (Variables|Components|SetAura%20Sphere 0)))))

(event Collision|EventActorBeginOverlap
  (params (OtherActor :type Actor%20Object%20Reference)))

(event EventTick
  (params (DeltaSeconds :type Float%20%28single-precision%29))
  (Variables|Default|SetNiagaraComp "/Game/Blueprint/WindEffect.WindEffect")
  (Class|BlueprintCameraVariableTableFunctionLibrary|SetFloatCameraVariable :Value 1e+01))

(fn ConstructionScript)